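; Physics-driven ball actor for what appears to be a Pong-style game with an AI opponent.
; On BeginPlay it registers itself with the AI_BP actor, then launches its sphere along X, with Switch choosing the direction and a random Y adding angle.
; Each hit plays a beep and raises BallSpeed, clamping physics velocity to exactly that magnitude.
; When destroyed, it asks its spawner reference to spawn another ball.
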(event EventBeginPlay
  (bind _sphere (Variables|Default|GetSphere))
  (bind _returnvalue (Actor|GetActorOfClass "/Game/Blueprints/AI_BP.AI_BP_C"))
  (bind _output_get (Variables|Default|SetAI_Ref _returnvalue))
  (Variables|/Game/Blueprints/AI_BP.AI_BP_C|SetBallRef _output_get self)
  (if (Variables|Default|GetSwitch)
    (Physics|AddImpulse _sphere (Math|Vector|MakeVector 1e+03 (Math|Conversions|ToFloat(Integer) (Math|Random|RandomIntegerinRange -360 360)) 0.0) "None" true)
    (else
      (Physics|AddImpulse _sphere (Math|Vector|MakeVector -1e+03 (Math|Conversions|ToFloat(Integer) (Math|Random|RandomIntegerinRange -360 360)) 0.0) "None" true))))

(event Collision|EventHit
  (params (MyComp :type Primitive%20Component%20Object%20Reference) (Other :type Actor%20Object%20Reference) (OtherComp :type Primitive%20Component%20Object%20Reference) (bSelfMoved :type Boolean) (HitLocation :type Vector :default "0, 0, 0") (HitNormal :type Vector :default "0, 0, 0") (NormalImpulse :type Vector :default "0, 0, 0") (Hit :type Hit%20Result%20Structure%20%28by%20ref%29))
  (bind _sphere (Variables|Default|GetSphere))
  (Audio|PlaySoundatLocation "/Game/Sounds/ping_pong_8bit_beeep.ping_pong_8bit_beeep" (Transformation|GetActorLocation) "0, 0, 0" 1.0 1.0 0.0 0 0 0 0)
  (Variables|Default|SetBallSpeed (+ (Variables|Default|GetBallSpeed) 3e+01))
  (bind _returnvalue (Physics|GetPhysicsLinearVelocity _sphere "None"))
  (Physics|SetPhysicsLinearVelocity _sphere (Math|Vector|ClampVectorSize _returnvalue (Variables|Default|GetBallSpeed) (Variables|Default|GetBallSpeed)) false "None")
  (Physics|GetPhysicsLinearVelocity (Variables|Default|GetSphere) "None"))

(event EventDestroyed
  (Default|SpawnBall (Variables|Default|GetBallSpawnRef)))

(fn ConstructionScript)