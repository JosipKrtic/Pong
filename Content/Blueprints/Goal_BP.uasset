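; Goal trigger Blueprint for a Pong game that awards a point when the ball enters it.
; On BeginPlay it caches the player pawn as PongBP to reach the score HUD.
; When a BallBP overlaps its box, it destroys the ball and updates the opposing player's score, chosen by the Player1Goal flag.
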(event OnComponentBeginOverlap(Box)
  (params (OverlappedComponent :type Primitive%20Component%20Object%20Reference) (OtherActor :type Actor%20Object%20Reference) (OtherComp :type Primitive%20Component%20Object%20Reference) (OtherBodyIndex :type Integer) (bFromSweep :type Boolean) (SweepResult :type Hit%20Result%20Structure%20%28by%20ref%29))
  (bind _asball_bp (Utilities|Casting|CastToBallBP OtherActor))
  (Actor|DestroyActor _asball_bp)
  (if (Variables|Default|GetPlayer1Goal?)
    (Default|UpdatePlayer2Score (Variables|/Game/Blueprints/PongBP.PongBP_C|GetScoreHud (Variables|Default|GetPongRef)))
    (else
      (Default|UpdatePlayer1Score (Variables|/Game/Blueprints/PongBP.PongBP_C|GetScoreHud (Variables|Default|GetPongRef))))))

(event EventBeginPlay
  (bind _aspong_bp (Utilities|Casting|CastToPongBP (Game|Player|GetPlayerPawn 0)))
  (Variables|Default|SetPongRef _aspong_bp))

(fn ConstructionScript)